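; Player Blueprint for a side-view 2D character that walks, runs, crouches and jumps, using flipbook animation.
; Horizontal axis input adds movement along X and rotates the sprite to face the direction of travel.
; Independent crouch and run toggles set walk speed and call animation events that choose a movement or idle flipbook from current velocity.
; Flipbooks update only when a toggle is pressed, not during movement or jumping.
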(event Custom|Enable%20Walk%20Animation
  ;[1 1 1] Walking animation activation
  (Sprite|SetFlipbook (Variables|Default|GetSprite) (select (> (Math|Vector|VectorLength (Transformation|GetVelocity)) 0.0) "/Game/Flipbooks/PlayerWalk.PlayerWalk" "/Game/Flipbooks/PlayerIdle.PlayerIdle")))

(event Custom|Enable%20Run%20Animation
  ;[1 1 1] Activate animation of running
  (Sprite|SetFlipbook (Variables|Default|GetSprite) (select (> (Math|Vector|VectorLength (Transformation|GetVelocity)) 0.0) "/Game/Flipbooks/PlayerRun.PlayerRun" "/Game/Flipbooks/PlayerIdle.PlayerIdle")))

(event Custom|Enable%20Crouch%20Animation
  ;[1 1 1] Activate animation of crouching
  (Sprite|SetFlipbook (Variables|Default|GetSprite) (select (> (Math|Vector|VectorLength (Transformation|GetVelocity)) 0.0) "/Game/Flipbooks/PlayerCrouch.PlayerCrouch" "/Game/Flipbooks/PlayerIdle.PlayerIdle")))

(event Input|ActionEvents|InputActionJump
  (params (Key :type Key%20Structure :default "None"))
  ;[1 1 1] Handle Jump
  (:Pressed
    (Character|Jump)))

(event Input|ActionEvents|InputActionToggleCrouch
  (params (Key :type Key%20Structure :default "None"))
  (bind _charactermovement (Variables|Character|GetCharacterMovement))
  ;[1 1 1] Toggle crouch
  (:Pressed
    (bind _output_get (Variables|Default|SetIsCrouching (not (Variables|Default|GetIsCrouching))))
    (CallFunction|EnableCrouchAnimation)
    (if _output_get
      (Variables|/Script/Engine.CharacterMovementComponent|SetMaxWalkSpeed _charactermovement 5e+01)
      (CallFunction|EnableCrouchAnimation)
      (else
        (Variables|/Script/Engine.CharacterMovementComponent|SetMaxWalkSpeed _charactermovement 3e+02)
        (CallFunction|EnableWalkAnimation)))))

(event Input|ActionEvents|InputActionToggleRun
  (params (Key :type Key%20Structure :default "None"))
  (bind _charactermovement (Variables|Character|GetCharacterMovement))
  ;[1 1 1] Toggle run
  (:Pressed
    (bind _output_get (Variables|Default|SetIsRunning (not (Variables|Default|GetIsRunning))))
    (CallFunction|EnableRunAnimation)
    (if _output_get
      (Variables|/Script/Engine.CharacterMovementComponent|SetMaxWalkSpeed _charactermovement 1.2e+03)
      (CallFunction|EnableRunAnimation)
      (else
        (Variables|/Script/Engine.CharacterMovementComponent|SetMaxWalkSpeed _charactermovement 3e+02)
        (CallFunction|EnableWalkAnimation)))))

(event Input|AxisEvents|InputAxisMoveHorizontally
  (params (AxisValue :type Float%20%28single-precision%29))
  (bind _sprite (Variables|Default|GetSprite))
  ;[1 1 1] Handle movement
  (if (> AxisValue 0.0)
    (Transformation|SetRelativeRotation _sprite "0, 0, 0" false false)
    (Pawn|Input|AddMovementInput "1.000000,0.000000,0.000000" 1.0 false)
    (elif (< AxisValue 0.0)
      (Transformation|SetRelativeRotation _sprite "0.000000,180.000000,0.000000" false false)
      (Pawn|Input|AddMovementInput "-1.000000, 0, 0" 1.0 false))))

(fn ConstructionScript)