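; BP_Slope is a slope actor that sets its own rotation every tick.
; Tick combines CurrentRotation with a rotator built by MakeRotFromY from delta time plus the current pitch, converted to a vector, then applies it without teleporting physics.
; The construction script sets minimum and maximum rotations and a rotation time, but the graph never reads them or updates CurrentRotation.
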(event EventBeginPlay)

(event EventTick
  (params (DeltaSeconds :type Float%20%28single-precision%29))
  (Transformation|SetActorRotation (Math|Rotator|CombineRotators (Variables|Default|GetCurrentRotation) (Math|Rotator|MakeRotfromY (Math|Conversions|ToVector(Float) (+ DeltaSeconds (.Pitch (Math|Rotator|BreakRotator (Variables|Default|GetCurrentRotation)))))))))

(fn ConstructionScript
  (Variables|Default|SetMinRotation "0, 0, 0")
  (Variables|Default|SetMaxRotation "90.000000, 0, 0")
  (Variables|Default|SetRotationTimeSeconds 4))